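; Minion spawner actor that manages five child-actor spawn points for spawning minions of one configured tag and color against an enemy tag.
; On BeginPlay it passes tags and color to each BP_SpawnPoint, caches them in an array, and starts a looping timer at a set interval.
; SpawnMinion advances a wrapping index so the points take turns, delegating each spawn to the selected spawn point.
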(event `self.ReceiveBeginPlay`
  (`self.SetupSpawnPoints`)
  (`KismetSystemLibrary.K2_SetTimerDelegate` (`|CreateDelegate` :!event `SpawnMinion`) (`self.Interval`) true))

(fn `SetupSpawnPoints`
  (bind _output_get (set `self.SpawnPointsAsChildActors` (`|MakeArray` (`self.BP_SpawnPoint1`) (`self.BP_SpawnPoint2`) (`self.BP_SpawnPoint3`) (`self.BP_SpawnPoint4`) (`self.BP_SpawnPoint5`))))
  (for _array_element _output_get
    (bind _asbp_spawn_point (cast `/Game/Blueprints/BP_SpawnPoint` (`ChildActorComponent.ChildActor` _array_element)))
    (`/Game/Blueprints/BP_SpawnPoint.SetupSpawnPoint` _asbp_spawn_point (`self.MinionsTag`) (`self.EnemyTag`) (`self.Color`))
    (`KismetArrayLibrary.Array_Add` (`self.SpawnPointsAsActors`) _asbp_spawn_point)))

(fn `SpawnMinion`
  (bind _result (`/Engine/EditorBlueprintResources/StandardMacros.IncrementInt` (`self.CurrentSpawnPointIndex`))
    (:`  `
      (if (>= _result (`KismetArrayLibrary.Array_Length` (`self.SpawnPointsAsActors`)))
        (bind _output_get (set `self.CurrentSpawnPointIndex` 0))
        (`self.TriggerSpawner` _output_get)
        (else
          (`self.TriggerSpawner` _result))))))

(fn `TriggerSpawner`
  (params (Index :type Integer))
  (`/Game/Blueprints/BP_SpawnPoint.SpawnMinion` (`|GetArrayItem` (`self.SpawnPointsAsActors`) Index)))

(fn `UserConstructionScript`)
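; BP_SpawnPoint is a spawn point that creates AI minions at its own transform and assigns them to a side through tags.
; Setup stores the minion and enemy tags on the spawn point.
; SpawnMinion spawns regardless of collision, then, if the spawn is valid, sets the minion's EnemyTag and replaces its actor Tags with the single MinionTag.
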(fn `Setup`
  (params (MinionTag :type Name) (EnemyTag :type Name))
  (set `self.MinionTag` MinionTag)
  (set `self.EnemyTag` EnemyTag))

(fn `SpawnMinion`
  (bind _returnvalue (`|SpawnActorFromClass` "/Game/TopDown/Blueprints/AI_Minion.AI_Minion_C" (`self.GetTransform`) "AlwaysSpawn" "MultiplyWithRoot" null null))
  (`/Engine/EditorBlueprintResources/StandardMacros.IsValid` _returnvalue
    (:`Is Valid`
      (set `/Game/TopDown/Blueprints/AI_Minion.EnemyTag` (`self.EnemyTag`) _returnvalue)
      (set `Actor.Tags` (`|MakeArray` (`self.MinionTag`)) _returnvalue))))

(fn `UserConstructionScript`)